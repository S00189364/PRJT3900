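; Base weapon Blueprint for first-person guns, with a weapon mesh snapped to the arms' GripPoint socket.
; Events toggle firing and aim-down-sight flags, while separate functions handle shooting and reloading.
; Shooting requires a FirstPersonCharacter parent actor and ammo, spawning a projectile at the barrel along barrel rotation when aiming, otherwise camera rotation.
; Reloading refills the magazine from reserve ammo, allowing partial reloads.
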(event Custom|StartFiring
  (Variables|Default|SetIsWeaponFiring true))

(event Custom|StopFiring
  (Variables|Default|SetIsWeaponFiring false))

(event Custom|StartADS
  (Variables|Default|SetIsAimingDownSight true))

(event Custom|StopADS
  (Variables|Default|SetIsAimingDownSight false))

(fn ConstructionScript
  (Transformation|AttachComponentToComponent (Variables|Default|GetWeapons) (Variables|Default|GetArms) "GripPoint" "SnapToTarget" "SnapToTarget" "SnapToTarget" true))

(fn ShootingBullets
  (bind _asfirst_person_character (Utilities|Casting|CastToFirstPersonCharacter (Actor|GetParentActor)))
  (if (> (Variables|Default|GetCurrentAmmo) 0)
    (if (Variables|Default|GetIsAimingDownSight)
      (LocalVariables|SetBulletDirection (Transformation|GetWorldRotation (Variables|Default|GetWeaponBarrel)))
      (else
        (LocalVariables|SetBulletDirection (Transformation|GetWorldRotation (Variables|/Game/FirstPersonBP/FirstPersonCharacter.FirstPersonCharacter_C|GetFirstPersonCamera _asfirst_person_character)))))
    (Game|SpawnActorfromClass "/Game/FirstPersonBP/Blueprints/FirstPersonProjectile.FirstPersonProjectile_C" (Math|Transform|MakeTransform (Transformation|GetWorldLocation (Variables|Default|GetWeaponBarrel)) (LocalVariables|GetBulletDirection) "1,1,1") "Undefined" 0 0)
    (Variables|Default|SetCurrentAmmo (- (Variables|Default|GetCurrentAmmo) 1))))

(fn ReloadWeapon
  (bind _output_get (LocalVariables|SetBullet%20Difference (- (Variables|Default|GetMagSize) (Variables|Default|GetCurrentAmmo))))
  (if (>= (Variables|Default|GetMaxAmmo) _output_get)
    (Variables|Default|SetCurrentAmmo (Variables|Default|GetMagSize))
    (Variables|Default|SetMaxAmmo (- (Variables|Default|GetMaxAmmo) (LocalVariables|GetBullet%20Difference)))
    (else
      (Variables|Default|SetCurrentAmmo (+ (Variables|Default|GetCurrentAmmo) (Variables|Default|GetMaxAmmo)))
      (Variables|Default|SetMaxAmmo 0))))